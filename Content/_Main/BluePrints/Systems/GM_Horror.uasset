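; Horror game mode that tracks note count and escalates enemy speed as the count rises.
; CountNotes increments CantNotas and passes a higher velocity to CallSetVelocityEnemy at each of the first three notes.
; Counts beyond the third leave the speed unchanged, and the event graph holds no active logic.
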(event EventBeginPlay)

(event EventTick
  (params (DeltaSeconds :type Float%20%28single-precision%29)))

(fn ConstructionScript)

(fn CountNotes
  (bind _result (Math|Integer|IncrementInt (Variables|Default|GetCantNotas))
    (:%20%20
      (if (== _result 1)
        (Default|CallSetVelocityEnemy 5e+02)
        (elif (== _result 2)
          (Default|CallSetVelocityEnemy 7e+02)
          (elif (== _result 3)
            (Default|CallSetVelocityEnemy 9e+02)))))))