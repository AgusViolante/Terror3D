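; BP_AI_Base is an enemy that roams at random and kills the horror player character with a jumpscare on contact.
; On BeginPlay it chains AI moves to random navigable points nearby, repeating only after successful moves.
; Its walk speed follows a velocity event it binds on GM_Horror.
; A one-shot box overlap plays a scream, disables input, shows the player's animated jumpscare, destroys the enemy and flags the player dead.
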(event OnComponentBeginOverlap(Box)
  (params (OverlappedComponent :type Primitive%20Component%20Object%20Reference) (OtherActor :type Actor%20Object%20Reference) (OtherComp :type Primitive%20Component%20Object%20Reference) (OtherBodyIndex :type Integer) (bFromSweep :type Boolean) (SweepResult :type Hit%20Result%20Structure%20%28by%20ref%29))
  (bind _asbp_fcharacter_horror (Utilities|Casting|CastToBP_FCharacterHorror OtherActor))
  (Utilities|FlowControl|DoOnce false
    (:Completed
      (Audio|PlaySound2D "/Game/_Main/BluePrints/Sounds/220302__gabrielaupf__screaming_woman_horror.220302__gabrielaupf__screaming_woman_horror" 1.0 1.0 0.0 0 0)
      (Input|DisableInput _asbp_fcharacter_horror 0)
      (Rendering|SetVisibility (Variables|/Game/_Main/BluePrints/CharacterP/BP_FCharacterHorror.BP_FCharacterHorror_C|GetJumpscareREF _asbp_fcharacter_horror) true false)
      (Components|Animation|PlayAnimation (Variables|/Game/_Main/BluePrints/CharacterP/BP_FCharacterHorror.BP_FCharacterHorror_C|GetJumpscareREF _asbp_fcharacter_horror) "/Game/SKnight_modular/Skeleton_Knight_02/demo/animations/ThirdPerson_Jump.ThirdPerson_Jump" false)
      (Actor|DestroyActor)
      (Variables|/Game/_Main/BluePrints/CharacterP/BP_FCharacterHorror.BP_FCharacterHorror_C|Setdeath? _asbp_fcharacter_horror true))))

(event Custom|EnemyVelocity
  (params (Velocity :type Float%20%28double-precision%29))
  (Variables|/Script/Engine.CharacterMovementComponent|SetMaxWalkSpeed (Variables|Character|GetCharacterMovement) Velocity))

(event EventBeginPlay
  (bind _asgm_horror (Utilities|Casting|CastToGM_Horror (Game|GetGameMode)))
  (EventDispatchers|BindEventtoSetVelocityEnemy _asgm_horror (delegate Custom|EnemyVelocity))
  (bind _randomlocation (Class|NavigationSystemV1|GetRandomLocationinNavigableRadius (Transformation|GetActorLocation) 1e+03 0 0 :!label _label))
  (AI|AIMoveTo self _randomlocation 0 5.0 false
    (:OnSuccess
      (goto _label))))

(fn ConstructionScript)