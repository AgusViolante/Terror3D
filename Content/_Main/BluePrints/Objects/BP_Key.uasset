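; BP_Key is a key pickup actor that the player collects by interacting with it.
; On Interact, it passes its Key value to the player's AddKey function and then destroys itself.
; BeginPlay, overlap and Tick events are unused, so collection relies entirely on the interaction call.
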(event EventBeginPlay
  (|CallParentFunction) ; This node is disabled and will not be called.\nDrag off pins to build functionality.
)

(event Collision|EventActorBeginOverlap
  (params (OtherActor :type Actor%20Object%20Reference))
  (|CallParentFunction OtherActor) ; This node is disabled and will not be called.\nDrag off pins to build functionality.
)

(event EventTick
  (params (DeltaSeconds :type Float%20%28single-precision%29))
  (|CallParentFunction DeltaSeconds) ; This node is disabled and will not be called.\nDrag off pins to build functionality.
)

(event EventInteract
  (params (PlayerLocation :type Vector :default "0, 0, 0") (Player :type BP%20F%20Character%20Horror%20Object%20Reference))
  (Default|AddKey Player (Variables|Default|GetKey))
  (Actor|DestroyActor))

(fn ConstructionScript
  (|CallParentFunction))