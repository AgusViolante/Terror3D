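; BP_Door is an interactable, key-locked door that toggles open and closed when the player interacts with it.
; Interact checks that the player has the door's key, then ignores further input until the animation finishes.
; A dot product of the player-to-door direction and the door's forward vector picks the swing side, so it rotates away from or toward a signed 90-degree yaw.
; The OpenDoor timeline lerps the Puerta component's rotation, playing to open and reversing to close.
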(event EventBeginPlay
  (|CallParentFunction) ; This node is disabled and will not be called.\nDrag off pins to build functionality.
)

(event Collision|EventActorBeginOverlap
  (params (OtherActor :type Actor%20Object%20Reference))
  (|CallParentFunction OtherActor) ; This node is disabled and will not be called.\nDrag off pins to build functionality.
)

(event EventTick
  (params (DeltaSeconds :type Float%20%28single-precision%29))
  (|CallParentFunction DeltaSeconds) ; This node is disabled and will not be called.\nDrag off pins to build functionality.
)

(event EventInteract
  (params (PlayerLocation :type Vector :default "0, 0, 0") (Player :type BP%20F%20Character%20Horror%20Object%20Reference))
  (bind _playerkeys (Default|HasKey Player (Variables|Default|GetKey)))
  (if _playerkeys
    ;[1 1 1] Abrir y cerrar la puerta
    (if (Variables|Default|GetAnimationFinish)
      (Variables|Default|SetAnimationFinish false)
      (bind _output_get (Variables|Default|SetIsInteractableActive (not (Variables|Default|GetIsInteractableActive))))
      (if _output_get
        (Variables|Default|SetTargetRotation (Math|Float|SelectFloat 9e+01 -9e+01 (>= (Math|Vector|DotProduct (Math|Vector|GetUnitDirection(Vector) PlayerLocation (Transformation|GetActorLocation)) (Transformation|GetActorForwardVector)) 0.0)))
        (bind _alpha (Timeline|OpenDoor Play)
          (:Update
            (Transformation|SetRelativeRotation (Variables|Default|GetPuerta) (Math|Rotator|MakeRotator 0.0 0.0 (Math|Float|Lerp 0.0 (Variables|Default|GetTargetRotation) _alpha)) false false))
          (:Finished
            (Variables|Default|SetAnimationFinish true)))
        (else
          (Timeline|OpenDoor Reverse))))))

(fn ConstructionScript
  (|CallParentFunction))