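; BP_Note is an interactable paper note that the player picks up and reads in a horror game.
; On Interact it flags the player as reading, adds its text to their notes and removes its interaction widget.
; The paper sprite attaches to the player's ArrowNote keeping world transform, then a timeline lerps it into reading position.
; When the animation finishes, the HUD displays the text and GM_Horror updates the note count.
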(event EventBeginPlay
  (|CallParentFunction)
  (bind _asgm_horror (Utilities|Casting|CastToGM_Horror (Game|GetGameMode)))
  (Variables|Default|SetGameMode _asgm_horror))

(event Collision|EventActorBeginOverlap
  (params (OtherActor :type Actor%20Object%20Reference))
  (|CallParentFunction OtherActor) ; This node is disabled and will not be called.\nDrag off pins to build functionality.
)

(event EventTick
  (params (DeltaSeconds :type Float%20%28single-precision%29))
  (|CallParentFunction DeltaSeconds) ; This node is disabled and will not be called.\nDrag off pins to build functionality.
)

(event EventInteract
  (params (PlayerLocation :type Vector :default "0, 0, 0") (Player :type BP%20F%20Character%20Horror%20Object%20Reference))
  (bind _papersprite (Variables|Default|GetPaperSprite))
  (Default|PlayerReadingNote Player true)
  (bind _cantnotes (Default|AddNotes Player (Variables|Default|GetText)))
  (Variables|/Game/_Main/BluePrints/CharacterP/BP_FCharacterHorror.BP_FCharacterHorror_C|SetCantNotes Player _cantnotes)
  (Transformation|AttachComponentToComponent _papersprite (Variables|/Game/_Main/BluePrints/CharacterP/BP_FCharacterHorror.BP_FCharacterHorror_C|GetArrowNote Player) "None" "KeepWorld" "KeepWorld" "KeepWorld" true)
  (Variables|Default|SetSpriteTransform (Transformation|GetRelativeTransform _papersprite))
  (Components|DestroyComponent (Variables|Default|GetWidgetInteract))
  (bind _alpha (Timeline|NoteTimeline Play)
    (:Update
      (Transformation|SetRelativeTransform (Variables|Default|GetPaperSprite) (Math|Transform|Lerp(Transform) (Variables|Default|GetSpriteTransform) (Math|Transform|MakeTransform "0, 0, 0" "0.000000,0.000000,90.000000" (.Scale (Math|Transform|BreakTransform (Variables|Default|GetSpriteTransform)))) _alpha) false false))
    (:Finished
      (bind _hud (Class|INTHUD|HUDReference(Message) (HUD|GetHUD (Game|GetPlayerController 0))))
      (Default|ToggleNote (Variables|/Game/_Main/BluePrints/UI/HUD/BP_HUD.BP_HUD_C|GetHudWidget _hud) true (Variables|Default|GetText))
      (Default|CountNotes (Variables|Default|GetGameMode)))))

(fn ConstructionScript
  (|CallParentFunction))

(fn HUDReference
  (return 0))